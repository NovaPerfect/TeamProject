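; BP_Interact is an interactable actor that shows a widget when the first-person character comes within range.
; A sphere overlap makes the widget visible unless the character is already grabbing an object, and ending the overlap hides it.
; The grab state is checked only on overlap begin, and the end event hides the widget for any actor.
; The construction script sets the sphere's world Y scale from SphereScale, reusing its relative X and Z.
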(event OnComponentBeginOverlap(Sphere)
  (params (OverlappedComponent :type Primitive%20Component%20Object%20Reference) (OtherActor :type Actor%20Object%20Reference) (OtherComp :type Primitive%20Component%20Object%20Reference) (OtherBodyIndex :type Integer) (bFromSweep :type Boolean) (SweepResult :type Hit%20Result%20Structure%20%28by%20ref%29))
  (bind _widget (Variables|Default|GetWidget))
  (bind _asbp_first_person_character (Utilities|Casting|CastToBP_FirstPersonCharacter OtherActor))
  (if (Variables|/Game/FirstPerson/Blueprints/BP_FirstPersonCharacter.BP_FirstPersonCharacter_C|GetisGrabbingObject? _asbp_first_person_character)
    (Rendering|SetVisibility _widget false false)
    (else
      (Rendering|SetVisibility _widget true false))))

(event OnComponentEndOverlap(Sphere)
  (params (OverlappedComponent :type Primitive%20Component%20Object%20Reference) (OtherActor :type Actor%20Object%20Reference) (OtherComp :type Primitive%20Component%20Object%20Reference) (OtherBodyIndex :type Integer))
  (Rendering|SetVisibility (Variables|Default|GetWidget) false false))

(fn ConstructionScript
  (bind _sphere (Variables|Default|GetSphere))
  (bind _relativescale3d (Variables|/Script/Engine.SceneComponent|GetRelativeScale3D _sphere))
  (Transformation|SetWorldScale3D _sphere (Math|Vector|MakeVector (.x _relativescale3d) (.y (Variables|Default|GetSphere%20Scale)) (.z _relativescale3d))))