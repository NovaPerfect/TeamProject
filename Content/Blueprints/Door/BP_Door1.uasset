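; BP_Door1 is a door actor that rotates about its yaw when its DoorRotate event is called.
; The RotateNames enum selects one of four timelines, named for quarter-turn swings between fixed angles, each driving the actor's world yaw on update.
; The construction script applies the Door mesh variable to the SMDoorOffice component.
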(event EventDoorRotate
  (switch string (Utilities|String|EnumtoString (Variables|Default|GetRotateNames))
    (:From%200%20to%20-90
      (bind _rotation (Timeline|Timeline Play)
        (:Update
          (Transformation|SetActorRotation (Math|Rotator|MakeRotator 0.0 0.0 _rotation)))))
    (:From%2090%20to%200
      (bind _rotation_2 (Timeline|Timeline_0 Play)
        (:Update
          (Transformation|SetActorRotation (Math|Rotator|MakeRotator 0.0 0.0 _rotation_2)))))
    (:From%20-90%20to%20-180
      (bind _rotation_3 (Timeline|Timeline_1 Play)
        (:Update
          (Transformation|SetActorRotation (Math|Rotator|MakeRotator 0.0 0.0 _rotation_3)))))
    (:From%20180%20to%2090
      (bind _rotation_4 (Timeline|Timeline_2 Play)
        (:Update
          (Transformation|SetActorRotation (Math|Rotator|MakeRotator 0.0 0.0 _rotation_4)))))))

(fn ConstructionScript
  (Components|StaticMesh|SetStaticMesh (Variables|Default|GetSM_DoorOffice) (Variables|Default|GetDoor)))